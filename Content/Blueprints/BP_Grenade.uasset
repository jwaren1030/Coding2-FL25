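; BP_Grenade is a grenade item that can be picked up, held and dropped, with placeholder use actions.
; Pickup attaches it to the given skeletal mesh's hand_r socket and disables the Sphere's collision.
; Drop detaches it, restores collision and briefly simulates physics on the Sphere before switching simulation off after a delay.
; Primary and secondary use only print throw and drop explosion messages, with no explosion logic.
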(event `self.Pickup`
  (params (SkeletalMesh :type "SkeletalMeshComponent Object Reference"))
  ; Pickup Function
  (`KismetSystemLibrary.PrintText` (`|FormatText` "{name} is getting picked up and attached to {mesh}." "Grenade" _))
  (`self.K2_AttachToComponent` SkeletalMesh "hand_r" "SnapToTarget" "SnapToTarget" "SnapToTarget")
  (`PrimitiveComponent.SetCollisionEnabled` (`self.Sphere`) "NoCollision"))

(event `self.UsePrimary`
  ; UsePrimary Function
  (`KismetSystemLibrary.PrintText` "Throw... Delay... Boom (Use Primary)"))

(event `self.UseSecondary`
  ; UseSecondary Function
  (`KismetSystemLibrary.PrintText` "Drop... Boom! (Use Secondary"))

(event `self.Drop`
  (bind _sphere (`self.Sphere`))
  ; Drop Function
  (`self.K2_DetachFromActor` "KeepWorld" "KeepWorld" "KeepWorld")
  (`PrimitiveComponent.SetSimulatePhysics` _sphere true)
  (`PrimitiveComponent.SetCollisionEnabled` _sphere "QueryAndPhysics")
  (`KismetSystemLibrary.Delay` 2.0)
  (`PrimitiveComponent.SetSimulatePhysics` _sphere false))

(fn `UserConstructionScript`)