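; BP_LoopsAndLists is a Blueprint that demonstrates loops and array handling through on-screen debug prints.
; BeginPlay starts DelayLoop, a custom event that prints and increments a counter, waits on a Delay, calls PrintColors, then calls itself again indefinitely.
; PrintColors loops over the Textcolors array, printing each index in a randomly picked array color, then a completion message.
; A Shuffle node on the array is left unconnected.
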(event `self.ReceiveBeginPlay`
  (`KismetSystemLibrary.PrintString` "LoopsAndLists is active")
  (`self.Delay loop`))

(event `Delay loop`
  (`KismetSystemLibrary.PrintString` (`KismetStringLibrary.Concat_StrStr` "Starting Delay Loop #" (`KismetStringLibrary.Conv_IntToString` (`self.DelayLoopCounter`))))
  (`/Engine/EditorBlueprintResources/StandardMacros.IncrementInt` (`self.DelayLoopCounter`)
    (:`  `
      (`KismetSystemLibrary.Delay` 1.0)
      (`self.Print Colors`)
      (`self.Delay loop`))))

(event `Print Colors`
  (bind _textcolors (`self.Textcolors`))
  (for (_ _array_index) _textcolors
    (`KismetSystemLibrary.PrintString` (`KismetStringLibrary.Concat_StrStr` "Print Color #" (`KismetStringLibrary.Conv_IntToString` _array_index)) true true (`KismetArrayLibrary.Array_Random` _textcolors)))
  (`KismetSystemLibrary.PrintString` "We are done printing colors" true true (struct :`A` 1.0)))

(fn `UserConstructionScript`)