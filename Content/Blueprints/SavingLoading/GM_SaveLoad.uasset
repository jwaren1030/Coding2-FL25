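; GM_SaveLoad is a game mode that saves and loads player stats through an SG_PlayerStats save game.
; On BeginPlay it loads the PlayerSave slot and copies the saved stamina onto the BP_ThirdPersonCharacter, or creates an empty save object if none exists.
; SavePlayerStats writes the held save object to that slot, relying on other code to update its values first, and prints the result.
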(event `self.ReceiveBeginPlay`
  (`KismetSystemLibrary.PrintString` "Loading the SavLoad Game Mode" true true (struct :`R` 1.0 :`B` 0.057231 :`A` 1.0) 10.0)
  (`self.Load Player Stats`))

(event `Load Player Stats`
  (bind _returnvalue (`GameplayStatics.DoesSaveGameExist` "PlayerSave"))
  (if _returnvalue
    (bind _returnvalue_2 (`GameplayStatics.LoadGameFromSlot` "PlayerSave"))
    (bind _assg_player_stats (cast `/Game/Blueprints/SavingLoading/SG_PlayerStats` _returnvalue_2))
    (set `self.SG_PlayerStats` _assg_player_stats)
    (bind _asbp_third_person_character (cast `/Game/ThirdPerson/Blueprints/BP_ThirdPersonCharacter` (`GameplayStatics.GetPlayerCharacter` 0)))
    (set `/Game/ThirdPerson/Blueprints/BP_ThirdPersonCharacter.Stamina` (`/Game/Blueprints/SavingLoading/SG_PlayerStats.Stamina` (`self.SG_PlayerStats`)) _asbp_third_person_character)
    (`KismetSystemLibrary.PrintString` "PlayerStats have been loaded" true true (struct :`R` 1.0 :`B` 0.216168 :`A` 1.0))
    (else
      (bind _returnvalue_3 (`GameplayStatics.CreateSaveGameObject` "/Game/Blueprints/SavingLoading/SG_PlayerStats.SG_PlayerStats_C"))
      (set `self.SG_PlayerStats` _returnvalue_3) ; Set this variable so that the Player can edit these values
    )))

(event `Save Player Stats`
  (bind _returnvalue (`GameplayStatics.SaveGameToSlot` (`self.SG_PlayerStats`) "PlayerSave"))
  (if _returnvalue
    (`KismetSystemLibrary.PrintText` "Player Stats Written to Save Game File" true true (struct :`R` 1.0 :`B` 0.703602 :`A` 1.0))
    (else
      (`KismetSystemLibrary.PrintText` "Player Stats Couldn't Be Written to Save Game File"))))

(fn `UserConstructionScript`)