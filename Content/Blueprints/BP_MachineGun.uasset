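; BP_MachineGun is a machine gun pickup that can be attached to a character's hand, used and dropped.
; Pickup snaps it to the hand_r socket of the given skeletal mesh and disables collision on the gun body.
; UsePrimary only prints placeholder "Pew Pew Pew" text, with no firing logic.
; Drop detaches it, restores collision and simulates physics briefly before switching physics off after a delay.
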(event `/Game/Blueprints/BPI_Item.Pickup`
  (params (SkeletalMesh :type "SkeletalMeshComponent Object Reference"))
  ; Pickup Function
  (`KismetSystemLibrary.PrintText` (`|FormatText` "{name} is getting picked up and attached to {mesh}." "Machine Gun" SkeletalMesh))
  (`self.K2_AttachToComponent` SkeletalMesh "hand_r" "SnapToTarget" "SnapToTarget" "SnapToTarget")
  (`PrimitiveComponent.SetCollisionEnabled` (`self.MachineGunBody`) "NoCollision"))

(event `/Game/Blueprints/BPI_Item.UsePrimary`
  ; UsePrimary Function
  (`KismetSystemLibrary.PrintText` "Pew Pew Pew"))

(event `/Game/Blueprints/BPI_Item.Drop`
  (bind _machinegunbody (`self.MachineGunBody`))
  ; Drop Function
  (`self.K2_DetachFromActor` "KeepWorld" "KeepWorld" "KeepWorld")
  (`PrimitiveComponent.SetSimulatePhysics` _machinegunbody true)
  (`PrimitiveComponent.SetCollisionEnabled` _machinegunbody "QueryAndPhysics")
  (`KismetSystemLibrary.Delay` 2.0)
  (`PrimitiveComponent.SetSimulatePhysics` (`self.MachineGunBody`) false))

(fn `UserConstructionScript`)