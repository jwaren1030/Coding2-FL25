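; BP_Key is a collectible key pickup for the third-person character.
; When the character overlaps its sphere, the key destroys itself, increments the character's NumKeys count and prints the new total as a debug message.
; It also prints a debug message when it spawns.
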(event `self.ReceiveBeginPlay`
  (`KismetSystemLibrary.PrintString` "Key was created"))

(event `self.Sphere1.OnComponentBeginOverlap`
  (params (OverlappedComponent :type "PrimitiveComponent Object Reference") (OtherActor :type "Actor Object Reference") (OtherComp :type "PrimitiveComponent Object Reference") (OtherBodyIndex :type Integer) (bFromSweep :type Boolean) (SweepResult :type "HitResult Structure (by ref)"))
  (bind _asbp_third_person_character (cast `/Game/ThirdPerson/Blueprints/BP_ThirdPersonCharacter` OtherActor))
  (bind _output_get (set `self.Player` _asbp_third_person_character))
  (`self.K2_DestroyActor`)
  (bind _result (`/Engine/EditorBlueprintResources/StandardMacros.IncrementInt` (`/Game/ThirdPerson/Blueprints/BP_ThirdPersonCharacter.NumKeys` _asbp_third_person_character))
    (:`  `
      (bind _output_get_2 (set `/Game/ThirdPerson/Blueprints/BP_ThirdPersonCharacter.NumKeys` _result _output_get))
      (`KismetSystemLibrary.PrintString` (`KismetStringLibrary.Concat_StrStr` "You got a key! You have " (`KismetStringLibrary.Conv_IntToString` _output_get_2) " keys!")))))

(fn `UserConstructionScript`)