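; BP_CameraDoor is a door that opens by sliding down, either on request with a camera cutscene or by spending a player key.
; OpenDoor blends the view to the door, plays a timeline to lower it, then returns the camera to the passed-in target.
; Overlapping its sphere with a key consumes one and lowers the door without the camera shift.
; Opened doors register in GM_SaveLoad's level state, and AlreadyOpened restores the lowered position.
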(event `OpenDoor`
  (params (NewViewTarget :type "Actor Object Reference"))
  (if (not (`self.Opened`))
    (`PlayerController.SetViewTargetWithBlend` (`GameplayStatics.GetPlayerController` 0) self (`self.Blend Time`) "VTBlend_Cubic" 0.0 true)
    (`KismetSystemLibrary.Delay` (`self.Blend Time`))
    (bind (_direction _newtrack_0) (`Timeline|Timeline`)
      (:`Update`
        (`SceneComponent.K2_SetRelativeLocation` (`self.Door`) (`KismetMathLibrary.VLerp` (0.0 0.0 150.0) (0.0 0.0 -130.0) _newtrack_0) false false)
        (bind _asgm_save_load (cast `/Game/Blueprints/SavingLoading/GM_SaveLoad` (`GameplayStatics.GetGameMode`)))
        (`KismetArrayLibrary.Array_AddUnique` (`/Game/Blueprints/SavingLoading/SG_LevelState.Opened Doors` (`/Game/Blueprints/SavingLoading/GM_SaveLoad.SG_LevelState` _asgm_save_load)) self)
        (set `self.Opened` true))
      (:`Finished`
        (`KismetSystemLibrary.Delay` 2.0) ; waiting 2 seconds while the door opens
        (`PlayerController.SetViewTargetWithBlend` (`GameplayStatics.GetPlayerController` 0) NewViewTarget (/ (`self.Blend Time`) 2.0) "VTBlend_Cubic" 0.0 false) ; shift camera back to player
      ))))

(event `AlreadyOpened`
  (`KismetSystemLibrary.PrintText` "Door State Loaded" true true (struct :`R` 1.0 :`G` 0.915872 :`A` 1.0))
  (set `self.Opened` true)
  (`SceneComponent.K2_SetRelativeLocation` (`self.Door`) (0.0 0.0 -130.0) false false))

(event `self.Sphere.OnComponentBeginOverlap`
  (params (OverlappedComponent :type "PrimitiveComponent Object Reference") (OtherActor :type "Actor Object Reference") (OtherComp :type "PrimitiveComponent Object Reference") (OtherBodyIndex :type Integer) (bFromSweep :type Boolean) (SweepResult :type "HitResult Structure (by ref)"))
  (if (not (`self.Opened`))
    (bind _asbp_third_person_character (cast `/Game/ThirdPerson/Blueprints/BP_ThirdPersonCharacter` OtherActor))
    (bind _output_get (set `self.Player` _asbp_third_person_character))
    (bind _numkeys (`/Game/ThirdPerson/Blueprints/BP_ThirdPersonCharacter.NumKeys` _output_get))
    (if (> _numkeys 0)
      (bind _result (`/Engine/EditorBlueprintResources/StandardMacros.DecrementInt` _numkeys)
        (:`  `
          (set `/Game/ThirdPerson/Blueprints/BP_ThirdPersonCharacter.NumKeys` _result _output_get)
          (`KismetSystemLibrary.PrintString` "You open the door")
          (bind (_direction _newtrack_0) (`Timeline|Timeline_0`)
            (:`Update`
              (`SceneComponent.K2_SetRelativeLocation` (`self.Door`) (`KismetMathLibrary.VLerp` (0.0 0.0 150.0) (0.0 0.0 -130.0) _newtrack_0) false false)
              (bind _asgm_save_load (cast `/Game/Blueprints/SavingLoading/GM_SaveLoad` (`GameplayStatics.GetGameMode`)))
              (`KismetArrayLibrary.Array_AddUnique` (`/Game/Blueprints/SavingLoading/SG_LevelState.Opened Doors` (`/Game/Blueprints/SavingLoading/GM_SaveLoad.SG_LevelState` _asgm_save_load)) self)
              (set `self.Opened` true)))))
      (else
        (`KismetSystemLibrary.PrintString` "You need a key!")))))

(fn `UserConstructionScript`)