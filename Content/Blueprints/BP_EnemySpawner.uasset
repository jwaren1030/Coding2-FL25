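; BP_EnemySpawner populates the level with BP_AiMoveTo enemies at BeginPlay.
; It finds every BP_EnemySpawnPoint and gives each a weighted chance, favouring success, to spawn an enemy at its transform.
; Each spawned enemy receives a random skeletal mesh and name from the spawner's arrays.
; AIName and the displayed name text are drawn by separate random picks, so they can differ.
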(event `self.ReceiveBeginPlay`
  (bind _outitem (`KismetArrayLibrary.Array_Random` (`self.NameArray`)))
  (`KismetSystemLibrary.PrintString` "Enemy Spawner is Active")
  (bind _outactors (`GameplayStatics.GetAllActorsOfClass` "/Game/Blueprints/BP_EnemySpawnPoint.BP_EnemySpawnPoint_C"))
  (for _array_element _outactors
    (if (`KismetMathLibrary.RandomBoolWithWeight` 0.75)
      (bind _returnvalue (`|SpawnActorFromClass` "/Game/AI_Blueprints/BP_AiMoveTo.BP_AiMoveTo_C" (`self.GetTransform` _array_element) "Undefined" "MultiplyWithRoot" null null)) ; Spawn actor from class
      (bind _asbp_ai_move_to (cast `/Game/AI_Blueprints/BP_AiMoveTo` _returnvalue))
      (set `/Game/AI_Blueprints/BP_AiMoveTo.AI_Name` _outitem _asbp_ai_move_to)
      (`TextRenderComponent.K2_SetText` (`/Game/AI_Blueprints/BP_AiMoveTo.AI Name Text` _asbp_ai_move_to) (`KismetTextLibrary.Conv_StringToText` _outitem))
      (`SkeletalMeshComponent.SetSkeletalMeshAsset` (`Character.Mesh` _asbp_ai_move_to) (`KismetArrayLibrary.Array_Random` (`self.SkeletalMeshArray`))))))

(fn `UserConstructionScript`)